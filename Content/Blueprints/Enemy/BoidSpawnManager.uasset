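; Boid spawn manager that creates a ring of eight Boid AI pawns around its own location when play begins.
; A loop rotates a forward vector in equal yaw steps and scales it by SpawnRadius to get each spawn point.
; Each Boid spawns yawed toward the world origin, treated as the map center, rather than toward the spawner.
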(event EventBeginPlay
  (for _index (range 0 7)
    (AI|SpawnAIFromClass "/Game/Blueprints/Enemy/Boid.Boid_C" 0 (+ (* (Math|Rotator|GetRotationXVector (Math|Rotator|MakeRotator 0.0 0.0 (* _index 45.0))) (Variables|Default|GetSpawnRadius)) (Transformation|GetActorLocation)) (Math|Rotator|MakeRotator 0.0 0.0 (.yaw (Math|Rotator|FindLookatRotation (+ (* (Math|Rotator|GetRotationXVector (Math|Rotator|MakeRotator 0.0 0.0 (* _index 45.0))) (Variables|Default|GetSpawnRadius)) (Transformation|GetActorLocation)) (Math|Vector|VectorZero)))) false 0)))

(fn ConstructionScript)